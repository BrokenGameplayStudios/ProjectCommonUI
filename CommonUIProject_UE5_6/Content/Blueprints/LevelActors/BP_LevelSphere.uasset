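; BP_LevelSphere is an interactable level actor whose static mesh grows each time it receives the SendInteractableMessage event.
; The construction script caches the mesh's world scale in NewScale.
; Each message multiplies that stored value by a fixed factor and applies it as the new world scale, so growth compounds with no upper limit.
; BeginPlay, overlap and Tick are unused.
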(event `/Game/Data/BPI_UI.SendInteractableMessage`
  (set `self.New Scale` (* (`self.New Scale`) (1.1 1.1 1.1)))
  (`SceneComponent.SetWorldScale3D` (`self.StaticMesh`) (`self.New Scale`)))

(fn `UserConstructionScript`
  (`parent.UserConstructionScript`)
  (set `self.New Scale` (`SceneComponent.K2_GetComponentScale` (`self.StaticMesh`))))